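; Music analyzer actor that plays a track, animates frequency and amplitude equalizer bars, and feeds both spectra to the Wheel_BP death wheel.
; The construction script builds tinted bar rows, which a looping timer rescales from sound-analysis plugin, random or saved values.
; Each update appends values to an array loaded from the Frequency save slot and written back late in play, allowing time-stamped replay without live analysis.
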(event `self.ReceiveBeginPlay`
  (`|ExecutionSequence`
    (:`then_0`
      (bind _returnvalue (`GameplayStatics.DoesSaveGameExist` "Frequency"))
      (if _returnvalue
        ;[1 1 1] Load Game if Any
        (bind _returnvalue_2 (`GameplayStatics.LoadGameFromSlot` "Frequency"))
        (bind _assaved_frequencies (cast `/Game/Blueprints/SavedFrequencies` _returnvalue_2))
        (bind _output_get (set `self.SaveBP` _assaved_frequencies))
        (set `self.Values` (`/Game/Blueprints/SavedFrequencies.SavedValues` _output_get))
        (else
          ;[1 1 1] Save Game if Not
          (bind _returnvalue_3 (`GameplayStatics.CreateSaveGameObject` "/Game/Blueprints/SavedFrequencies.SavedFrequencies_C"))
          (bind _assaved_frequencies_2 (cast `/Game/Blueprints/SavedFrequencies` _returnvalue_3))
          (bind _output_get_2 (set `self.SaveBP` _assaved_frequencies_2))
          (`GameplayStatics.SaveGameToSlot` _output_get_2 "Frequency"))))
    (:`then_1`
      (bind _outactors (`GameplayStatics.GetAllActorsOfClass` "/Game/Blueprints/Wheel_BP.Wheel_BP_C"))
      (set `self.DeathWheel` (`KismetArrayLibrary.Array_Get` _outactors)))
    (:`then_2`
      (`KismetSystemLibrary.K2_SetTimerDelegate` (delegate `UpdateEqualizer`) 0.1 true)
      (`GameplayStatics.PlaySoundAtLocation` (`self.Music`)))))

(event `UpdateEqualizer`
  (bind _spectrumwidth (`self.SpectrumWidth`))
  (bind _music (`self.Music`))
  (bind _gametime (`self.GameTime`))
  (bind _savebp (`self.SaveBP`))
  (bind _timelength (`self.TimeLength`))
  (bind (_item_gametime _item_frequencies _item_amplitude) (break `/Game/Blueprints/SpectrumTimeStamp` (`KismetArrayLibrary.Array_Get` (`self.Values`) (`self.ValuesIndex`))))
  (`|ExecutionSequence`
    (:`then_0`
      (switch `/Game/Blueprints/GeneratorTypes` (`self.ValuesOrigin`)
        (:`NewEnumerator0`
          ;[1 1 1] Generates Frequencies and Amplitude from Plugin
          (set `self.GameTime` (`KismetSystemLibrary.GetGameTimeInSeconds`))
          (`|ExecutionSequence`
            (:`then_0`
              (if (`self.Frequency`)
                (bind _outspectrum (`SoundVisualizationStatics.CalculateFrequencySpectrum` _music 0 _gametime _timelength _spectrumwidth))
                (bind _output_get (set `self.Frequencies` _outspectrum))
                (for (_array_element _array_index) _output_get
                  (bind _output_get_2 (set `self.FrequencyVariation` (* (`KismetMathLibrary.FClamp` _array_element 1.0 1000000.0) 0.04)))
                  (`SceneComponent.SetWorldScale3D` (`KismetArrayLibrary.Array_Get` (`self.FrequencyBarsArray`) _array_index) (`KismetMathLibrary.MakeVector` 1.0 1.0 _output_get_2)))))
            (:`then_1`
              (if (`self.Amplitude`)
                (bind _outamplitudes (`SoundVisualizationStatics.GetAmplitude` _music 0 _gametime _timelength _spectrumwidth))
                (bind _output_get_3 (set `self.Amplitudes` _outamplitudes))
                (for (_array_element_2 _array_index_2) _output_get_3
                  (bind _output_get_4 (set `self.FrequencyVariation` (* (`KismetMathLibrary.FClamp` _array_element_2 1.0 1000000.0) 0.001)))
                  (`SceneComponent.SetWorldScale3D` (`KismetArrayLibrary.Array_Get` (`self.AmplitudeBarsArray`) _array_index_2) (`KismetMathLibrary.MakeVector` 1.0 1.0 _output_get_4)))))))
        (:`NewEnumerator1`
          ;[1 1 1] Generates Frequencies and Amplitude Randomly
          (`self.RandomizeArrayRange` (`self.Frequencies`) 0.0 4.0)
          (`self.RandomizeArrayRange` (`self.Amplitudes`) 0.0 8.0)
          ;[1 1 1] Update Equalizer Bars
          (for (_array_element_3 _array_index_3) (`self.Frequencies`)
            (`SceneComponent.SetWorldScale3D` (`KismetArrayLibrary.Array_Get` (`self.FrequencyBarsArray`) _array_index_3) (`KismetMathLibrary.MakeVector` 1.0 1.0 _array_element_3))
            (for (_array_element_4 _array_index_4) (`self.Amplitudes`)
              (`SceneComponent.SetWorldScale3D` (`KismetArrayLibrary.Array_Get` (`self.AmplitudeBarsArray`) _array_index_4) (`KismetMathLibrary.MakeVector` 1.0 1.0 _array_element_4)))))
        (:`NewEnumerator2`
          ;[1 1 1] Read Saved Frequencies and Amplitudes
          (if (>= (`KismetSystemLibrary.GetGameTimeInSeconds`) _item_gametime)
            (`/Engine/EditorBlueprintResources/StandardMacros.IncrementInt` (`self.ValuesIndex`)
              (:`  `
                (set `self.Frequencies` _item_frequencies)
                (set `self.Amplitudes` _item_amplitude)
                ;[1 1 1] Update Equalizer Bars
                (for (_array_element_5 _array_index_5) (`self.Frequencies`)
                  (`SceneComponent.SetWorldScale3D` (`KismetArrayLibrary.Array_Get` (`self.FrequencyBarsArray`) _array_index_5) (`KismetMathLibrary.MakeVector` 1.0 1.0 (* (`KismetMathLibrary.FClamp` _array_element_5 1.0 1000000.0) 0.04)))
                  (for (_array_element_6 _array_index_6) (`self.Amplitudes`)
                    (`SceneComponent.SetWorldScale3D` (`KismetArrayLibrary.Array_Get` (`self.AmplitudeBarsArray`) _array_index_6) (`KismetMathLibrary.MakeVector` 1.0 1.0 (* (`KismetMathLibrary.FClamp` _array_element_6 1.0 1000000.0) 0.001)))))))))))
    (:`then_1`
      ;[1 1 1] Send Values to the Wheel
      (message `/Game/Blueprints/MusicSampleInterface.SampleUpdate` (`self.DeathWheel`) (`self.Frequencies`) (`self.Amplitudes`))
      (`KismetArrayLibrary.Array_Add` (`self.Values`) (make `/Game/Blueprints/SpectrumTimeStamp` (`self.GameTime`) (`self.Frequencies`) (`self.Amplitudes`))))
    (:`then_2`
      ;[1 1 1] Save Frequencies Values
      (if (> (`self.GameTime`) 400.0)
        (`/Engine/EditorBlueprintResources/StandardMacros.DoOnce` (not (`self.ShouldSave`))
          (:`Completed`
            (set `/Game/Blueprints/SavedFrequencies.SavedValues` (`self.Values`) _savebp)
            (`GameplayStatics.SaveGameToSlot` _savebp "Frequency")))))))

(fn `PrintSpectrumArray`
  (params (ArrayName :type String) (Array :type "Array of Float (double-precision)") (DisplayDuration :type "Float (double-precision)"))
  (for (_array_element _array_index) Array
    (`KismetSystemLibrary.PrintString` (`KismetStringLibrary.Concat_StrStr` ArrayName " " (`KismetStringLibrary.Conv_IntToString` _array_index) ": " (`KismetStringLibrary.Conv_DoubleToString` _array_element)) true true (struct :`G` 0.66 :`B` 1.0 :`A` 1.0) DisplayDuration))
  (return))

(fn `RandomizeArrayRange`
  (params (Array :type "Array of Float (double-precision)") (Min :type "Float (double-precision)") (Max :type "Float (double-precision)"))
  (for (_ _array_index) Array
    (`KismetArrayLibrary.Array_Set` Array _array_index (`KismetMathLibrary.RandomFloatInRange` Min Max)))
  (return))

(fn `UserConstructionScript`
  (bind _tintcolor (`self.TintColor`))
  (`|ExecutionSequence`
    (:`then_0`
      ;[1 1 1] Build Frequency Equalizer
      (for _index (range 1 (+ (`self.SpectrumWidth`) 1))
        (bind _returnvalue (`AddComponent|Static Mesh Component_8281` :`RelativeTransform` (`KismetMathLibrary.MakeTransform` (`KismetMathLibrary.MakeVector` 0.0 (* (+ (* _index 100.0) (* _index 10.0)) -1.0) (`self.Distance`)) (struct) (1.0 1.0 1.0))))
        (bind _returnvalue_2 (`PrimitiveComponent.CreateDynamicMaterialInstance` _returnvalue 0 "/Game/Materials/StepsMaterial.StepsMaterial"))
        (`MaterialInstanceDynamic.SetVectorParameterValue` _returnvalue_2 "ColorParameter" _tintcolor)
        (`KismetArrayLibrary.Array_Add` (`self.FrequencyBarsArray`) _returnvalue)))
    (:`then_1`
      ;[1 1 1] Build Amplitude Equalizer
      (for _index_2 (range 1 (+ (`self.SpectrumWidth`) 1))
        (bind _returnvalue_3 (`AddComponent|StaticMeshComponent_16580` :`RelativeTransform` (`KismetMathLibrary.MakeTransform` (`KismetMathLibrary.MakeVector` 0.0 (* (+ (* _index_2 100.0) (* _index_2 10.0)) -1.0)))))
        (bind _returnvalue_4 (`PrimitiveComponent.CreateDynamicMaterialInstance` _returnvalue_3 0 "/Game/Materials/StepsMaterial.StepsMaterial"))
        (`MaterialInstanceDynamic.SetVectorParameterValue` _returnvalue_4 "ColorParameter" _tintcolor)
        (`KismetArrayLibrary.Array_Add` (`self.AmplitudeBarsArray`) _returnvalue_3)))
    (:`then_2`
      ;[1 1 1] Initiate the Spectrum Tables
      (for _ (range (+ (`self.SpectrumWidth`) 1))
        (`KismetArrayLibrary.Array_Add` (`self.Frequencies`))
        (`KismetArrayLibrary.Array_Add` (`self.Amplitudes`))))))